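; LanternFollowBP is an actor, a lantern by its name, that follows player character 0.
; Each Tick it moves toward a target through VInterpTo, meant for smoothing though no delta time or speed is set, and rotates to face the player.
; The target adds a forward-vector offset to the player's location, but both multipliers are zero, so it resolves to the player's position.
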(event `self.ReceiveTick`
  (params (DeltaSeconds :type "Float (single-precision)"))
  (bind _returnvalue (`GameplayStatics.GetPlayerCharacter` 0))
  (bind _returnvalue_2 (`self.K2_GetActorLocation` _returnvalue))
  (`self.K2_SetActorLocationAndRotation` (`KismetMathLibrary.VInterpTo` (`self.K2_GetActorLocation`) (+ (* (* (`self.GetActorForwardVector` _returnvalue) 0.0) 0.0) _returnvalue_2)) (`KismetMathLibrary.FindLookAtRotation` (`self.K2_GetActorLocation`) _returnvalue_2)))

(fn `UserConstructionScript`)