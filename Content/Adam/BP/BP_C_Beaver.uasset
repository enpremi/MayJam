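; BP_C_Beaver is a beaver character actor that turns to face the player and can be absorbed.
; Every tick it sets its yaw toward the player pawn, offset by 90 degrees for the mesh orientation.
; Its Absorb event plays a timeline that drives a WPO material parameter across all body-part meshes, then destroys the actor when finished.
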(event `Absorb`
  (bind (_direction _wpo) (`Timeline|Timeline_0`)
    (:`Update`
      (`MeshComponent.SetScalarParameterValueOnMaterials` (`self.C_eye_R`) "WPO" _wpo)
      (`MeshComponent.SetScalarParameterValueOnMaterials` (`self.C_eye_L`) "WPO" _wpo)
      (`MeshComponent.SetScalarParameterValueOnMaterials` (`self.C_body_GeoSphere001`) "WPO" _wpo)
      (`MeshComponent.SetScalarParameterValueOnMaterials` (`self.C_beaverparts_Plane002`) "WPO" _wpo)
      (`MeshComponent.SetScalarParameterValueOnMaterials` (`self.C_beaverparts_Plane003`) "WPO" _wpo)
      (`MeshComponent.SetScalarParameterValueOnMaterials` (`self.C_beaverparts_Box004`) "WPO" _wpo))
    (:`Finished`
      (`self.K2_DestroyActor`))))

(event `self.ReceiveTick`
  (params (DeltaSeconds :type "Float (single-precision)"))
  (bind (_returnvalue_roll _returnvalue_pitch _returnvalue_yaw) (`KismetMathLibrary.BreakRotator` (`KismetMathLibrary.FindLookAtRotation` (`self.K2_GetActorLocation`) (`self.K2_GetActorLocation` (`GameplayStatics.GetPlayerPawn` 0)))))
  (`self.K2_SetActorRotation` (`KismetMathLibrary.MakeRotator` 0.0 0.0 (- _returnvalue_yaw 90.0))))

(fn `UserConstructionScript`)