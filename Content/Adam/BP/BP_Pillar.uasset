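; BP_Pillar is a shrine pillar where four animal souls (Panda, Beaver, Mole, Stag) are delivered to win the game.
; Each Deliver event plays a timeline that lights its own colored rune via a material vector parameter, then increments a shared soul count.
; At four souls it shows the Victory widget, then opens MenuMAP after a delay.
; A box overlap toggles the player character's NearShrine flag.
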(event `Deliver Panda`
  (bind (_direction _newtrack_0) (`Timeline|Timeline_1` :!via `PlayFromStart`)
    (:`Update`
      (`MeshComponent.SetVectorParameterValueOnMaterials` (`self.Pillar_LMain`) "First Rune" (* (1.0 2.0 5.0) (/ _newtrack_0 5.0))))
    (:`Finished`
      (set `self.Souls` (+ (`self.Souls`) 1) :!label _label)
      (`KismetSystemLibrary.Delay` 1.0)
      (if (== (`self.Souls`) 4)
        (bind _returnvalue (`|CreateWidget` "/Game/Jack/UI/Victory.Victory_C"))
        (`UserWidget.AddToViewport` _returnvalue 0)
        (`KismetSystemLibrary.Delay` 5.0)
        (`GameplayStatics.OpenLevel` "MenuMAP")))))

(event `Deliver Beaver`
  (bind (_direction _newtrack_0) (`Timeline|Timeline_0` :!via `PlayFromStart`)
    (:`Update`
      (`MeshComponent.SetVectorParameterValueOnMaterials` (`self.Pillar_LMain`) "Second Rune" (* (5.0 5.0 1.0) (/ _newtrack_0 5.0))))
    (:`Finished`
      (goto _label))))

(event `Deliver Mole`
  (bind (_direction _newtrack_0) (`Timeline|Timeline_2` :!via `PlayFromStart`)
    (:`Update`
      (`MeshComponent.SetVectorParameterValueOnMaterials` (`self.Pillar_LMain`) "Third Rune" (* (5.0 1.0 1.0) (/ _newtrack_0 5.0))))
    (:`Finished`
      (goto _label))))

(event `Deliver Stag`
  (bind (_direction _newtrack_0) (`Timeline|Timeline_3` :!via `PlayFromStart`)
    (:`Update`
      (`MeshComponent.SetVectorParameterValueOnMaterials` (`self.Pillar_LMain`) "Fourth Rune" (* (1.0 5.0 1.0) (/ _newtrack_0 5.0))))
    (:`Finished`
      (goto _label))))

(event `self.Box.OnComponentBeginOverlap`
  (params (OverlappedComponent :type "PrimitiveComponent Object Reference") (OtherActor :type "Actor Object Reference") (OtherComp :type "PrimitiveComponent Object Reference") (OtherBodyIndex :type Integer) (bFromSweep :type Boolean) (SweepResult :type "HitResult Structure (by ref)"))
  (bind _returnvalue (`GameplayStatics.GetPlayerPawn` 0))
  (if (and (`KismetStringLibrary.Contains` (`KismetSystemLibrary.GetObjectName` OtherComp) "cylinder") (== OtherActor _returnvalue))
    (set `/Game/OtterGames/OG_SideScrollerCharacter.NearShrine` true (cast `/Game/OtterGames/OG_SideScrollerCharacter` _returnvalue :!pure true))))

(event `self.Box.OnComponentEndOverlap`
  (params (OverlappedComponent :type "PrimitiveComponent Object Reference") (OtherActor :type "Actor Object Reference") (OtherComp :type "PrimitiveComponent Object Reference") (OtherBodyIndex :type Integer))
  (if (and (`KismetStringLibrary.Contains` (`KismetSystemLibrary.GetObjectName` OtherComp) "cylinder") (== OtherActor (`GameplayStatics.GetPlayerPawn` 0)))
    (set `/Game/OtterGames/OG_SideScrollerCharacter.NearShrine` false (cast `/Game/OtterGames/OG_SideScrollerCharacter` (`GameplayStatics.GetPlayerPawn` 0) :!pure true))))

(fn `UserConstructionScript`)