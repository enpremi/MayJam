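; BP_rocklauncher is an actor that continuously spawns BP_rock actors within a box-shaped area.
; On BeginPlay it starts a LaunchRock event that re-calls itself after a short fixed delay, forming an endless loop.
; Each spawn location is a random offset within the Box component's scaled extent, added to the actor's location.
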(event `self.ReceiveBeginPlay`
  (`self.Launch rock`))

(event `Launch rock`
  (bind _x (.x (`BoxComponent.GetScaledBoxExtent` (`self.Box`))))
  (bind _y (.y (`BoxComponent.GetScaledBoxExtent` (`self.Box`))))
  (bind _z (.z (`BoxComponent.GetScaledBoxExtent` (`self.Box`))))
  (`|SpawnActorFromClass` "/Game/Adam/BP/BP_rock.BP_rock_C" (`KismetMathLibrary.MakeTransform` (+ (`KismetMathLibrary.MakeVector` (`KismetMathLibrary.RandomFloatInRange` (* _x -1.0) _x) (`KismetMathLibrary.RandomFloatInRange` (* _y -1.0) _y) (`KismetMathLibrary.RandomFloatInRange` (* _z -1.0) _z)) (`self.K2_GetActorLocation`))) "Undefined" "OverrideRootScale" null null)
  (`KismetSystemLibrary.Delay` 1.5)
  (`self.Launch rock`))

(fn `UserConstructionScript`)