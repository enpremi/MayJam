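; Living tree actor that watches the player and plays a stomp attack animation when they enter its box.
; Each Tick drives morph targets: clamped world-space look-at yaw turns it left or right, while player distance controls mouth and eyes.
; The mouth opens as the player nears and the eyes close with distance; a bend-over morph is left unconnected.
; The construction script applies the chosen tree mesh and eye colour.
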(event `self.Box.OnComponentBeginOverlap`
  (params (OverlappedComponent :type "PrimitiveComponent Object Reference") (OtherActor :type "Actor Object Reference") (OtherComp :type "PrimitiveComponent Object Reference") (OtherBodyIndex :type Integer) (bFromSweep :type Boolean) (SweepResult :type "HitResult Structure (by ref)"))
  (if (== OtherActor (`GameplayStatics.GetPlayerPawn` 0))
    (`SkeletalMeshComponent.PlayAnimation` (`self.Tree_aniamted`) "/Game/Adam/Geo/stomp_attack.stomp_attack" false)))

(event `self.ReceiveTick`
  (params (DeltaSeconds :type "Float (single-precision)"))
  (bind _returnvalue (`GameplayStatics.GetPlayerPawn` 0))
  (bind _tree_aniamted (`self.Tree_aniamted`))
  (bind _tree_aniamted_2 (`self.Tree_aniamted`))
  (bind _tree_aniamted_3 (`self.Tree_aniamted`))
  (bind (_returnvalue_roll _returnvalue_pitch _returnvalue_yaw) (`KismetMathLibrary.BreakRotator` (`KismetMathLibrary.FindLookAtRotation` (`SceneComponent.K2_GetComponentLocation` _tree_aniamted) (`self.K2_GetActorLocation` _returnvalue))))
  (bind _returnvalue_2 (`KismetMathLibrary.FClamp` (+ _returnvalue_yaw 15.0) -50.0 50.0))
  (bind _returnvalue_3 (/ (`KismetMathLibrary.Abs` _returnvalue_2) 70.0))
  (bind _returnvalue_4 (- (/ (- (`KismetMathLibrary.FClamp` (`self.GetDistanceTo` (`ActorComponent.GetOwner` _tree_aniamted) _returnvalue) 200.0 400.0) 200.0) 200.0) 0.5))
  (`|ExecutionSequence`
    (:`then_1`
      (if (>= _returnvalue_2 0.0)
        (`SkeletalMeshComponent.SetMorphTarget` _tree_aniamted_3 "tree_full_turn_right" _returnvalue_3 true)
        (else
          (`SkeletalMeshComponent.SetMorphTarget` _tree_aniamted_3 "tree_full_turn_left" _returnvalue_3 true))))
    (:`then_2`
      (`SkeletalMeshComponent.SetMorphTarget` _tree_aniamted_2 "tree_full_open_mouth" (* _returnvalue_4 -2.0) true))
    (:`then_3`
      (`SkeletalMeshComponent.SetMorphTarget` _tree_aniamted_2 "tree_full_closed_eyes" _returnvalue_4 true))))

(event `self.ReceiveBeginPlay`)

(fn `UserConstructionScript`
  (bind _tree_aniamted (`self.Tree_aniamted`))
  (`SkinnedMeshComponent.SetSkinnedAssetAndUpdate` _tree_aniamted (`self.Tree_Type`) true)
  (`MeshComponent.SetVectorParameterValueOnMaterials` _tree_aniamted "Eyes_colour" (`KismetMathLibrary.Conv_LinearColorToVector` (`self.Eye_colour`))))